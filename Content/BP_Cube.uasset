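; BP_Cube is a roaming cube that gets painted on contact, spreading paint from the player through other cubes.
; It calls RandomRoam on BeginPlay.
; When hit by BP_Player or an already painted BP_Cube, it swaps its mesh material, sets its painted flag and calls End.
; RandomRoam and End are called here but not defined in this graph.
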(event `self.ReceiveBeginPlay`
  (`self.RandomRoam`))

(event `self.ReceiveHit`
  (params (MyComp :type "PrimitiveComponent Object Reference") (Other :type "Actor Object Reference") (OtherComp :type "PrimitiveComponent Object Reference") (bSelfMoved :type Boolean) (HitLocation :type "Vector Structure") (HitNormal :type "Vector Structure") (NormalImpulse :type "Vector Structure") (Hit :type "HitResult Structure (by ref)"))
  (cast `/Game/BP_Player` Other
    (:`then`
      (`PrimitiveComponent.SetMaterial` (`self.Mesh`) 0 "/Engine/MapTemplates/Materials/BasicAsset01.BasicAsset01")
      (set `self.IsPainted_0` true)
      (`self.end`))
    (:`CastFailed`
      (bind _asbp_cube (cast `/Game/BP_Cube` Other))
      (if (`/Game/BP_Parent.IsPainted_0` _asbp_cube)
        (`PrimitiveComponent.SetMaterial` (`self.Mesh`) 0 "/Engine/MapTemplates/Materials/BasicAsset01.BasicAsset01")
        (set `self.IsPainted_0` true)
        (`self.end`)))))

(fn `UserConstructionScript`)