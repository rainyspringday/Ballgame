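; BP_Parent is a base pawn Blueprint providing random roaming and an endgame notification.
; RandomRoam uses AI MoveTo toward a random reachable point around the actor and calls itself again on each successful arrival, with no handling for failed moves.
; The End function asks GM_MyGame to run EndgameCheck when the game is not paused.
; Nothing in this Blueprint calls either entry point.
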(event `RandomRoam`
  (`|AIMoveTo` self (`NavigationSystemV1.K2_GetRandomReachablePointInRadius` (`self.K2_GetActorLocation`) 2500.0 null null) null
    (:`OnSuccess`
      (`self.RandomRoam`))))

(fn `end`
  (if (not (`GameplayStatics.IsGamePaused`))
    (bind _asgm_my_game (cast `/Game/GM_MyGame` (`GameplayStatics.GetGameMode`)))
    (`/Game/GM_MyGame.Endgame_check` _asgm_my_game)))

(fn `UserConstructionScript`)