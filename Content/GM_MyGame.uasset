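; GM_MyGame is the game mode that ends the game once every BP_Cube and BP_ClearCube is painted.
; Each Tick it recounts unpainted clear cubes into Counter, then scans all cubes, checking clear cubes only when every regular one is painted.
; When both checks pass, it shows the WB_GameEnd widget and mouse cursor, pauses the game and destroys itself.
; The painted tallies reset at the end of each Tick sequence.
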(event `self.ReceiveTick`
  (params (DeltaSeconds :type "Float (single-precision)"))
  (`|ExecutionSequence`
    (:`then_0`
      (set `self.Counter` 0)
      (bind _outactors (`GameplayStatics.GetAllActorsOfClass` "/Game/BP_ClearCube.BP_ClearCube_C"))
      (for _array_element _outactors
        (if (not (`/Game/BP_ClearCube.IsPainted` _array_element))
          (`/Engine/EditorBlueprintResources/StandardMacros.IncrementInt` (`self.Counter`)))))
    (:`then_1`
      (bind _outactors_2 (`GameplayStatics.GetAllActorsOfClass` "/Game/BP_Cube.BP_Cube_C"))
      (for _array_element_2 _outactors_2
        (if (`/Game/BP_Cube.IsPainted` _array_element_2)
          (`/Engine/EditorBlueprintResources/StandardMacros.IncrementInt` (`self.EndgameCondition`))))
      (if (== (`self.EndgameCondition`) (`KismetArrayLibrary.Array_Length` _outactors_2))
        (bind _outactors_3 (`GameplayStatics.GetAllActorsOfClass` "/Game/BP_ClearCube.BP_ClearCube_C"))
        (for _array_element_3 _outactors_3
          (if (`/Game/BP_ClearCube.IsPainted` _array_element_3)
            (`/Engine/EditorBlueprintResources/StandardMacros.IncrementInt` (`self.EndgameCondition2`))))
        (if (== (`self.EndgameCondition2`) (`KismetArrayLibrary.Array_Length` _outactors_3))
          (bind _returnvalue (`|CreateWidget` "/Game/WB_GameEnd.WB_GameEnd_C"))
          (`UserWidget.AddToViewport` _returnvalue 0)
          (set `PlayerController.bShowMouseCursor` true (`GameplayStatics.GetPlayerController` 0))
          (`GameplayStatics.SetGamePaused` true)
          (`self.K2_DestroyActor`))))
    (:`then_2`
      (set `self.EndgameCondition` 0)
      (set `self.EndgameCondition2` 0))))

(fn `UserConstructionScript`)