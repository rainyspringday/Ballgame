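; BP_ClearCube is an AI-moved cube that wanders the level and spreads an unpainted state through collisions.
; A recursive roam event moves it to random reachable points, re-triggering only when a move succeeds.
; On hit, BP_Player paints it, while an unpainted ClearCube clears any BP_Cube it touches.
; Touching an unpainted ClearCube resets its own material and IsPainted flag.
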(event `RandomRoam`
  (`|AIMoveTo` self (`NavigationSystemV1.K2_GetRandomReachablePointInRadius` (`self.K2_GetActorLocation`) 2500.0 null null) null
    (:`OnSuccess`
      (`self.RandomRoam`))))

(event `self.ReceiveBeginPlay`
  (`self.RandomRoam`))

(event `self.ReceiveHit`
  (params (MyComp :type "PrimitiveComponent Object Reference") (Other :type "Actor Object Reference") (OtherComp :type "PrimitiveComponent Object Reference") (bSelfMoved :type Boolean) (HitLocation :type "Vector Structure") (HitNormal :type "Vector Structure") (NormalImpulse :type "Vector Structure") (Hit :type "HitResult Structure (by ref)"))
  (cast `/Game/BP_Player` Other
    (:`then`
      (`PrimitiveComponent.SetMaterial` (`self.Mesh`) 0 "/Engine/MapTemplates/Materials/BasicAsset01.BasicAsset01")
      (set `self.IsPainted` true))
    (:`CastFailed`
      (bind _asbp_cube (cast `/Game/BP_Cube` Other)
        (:`then`
          (if (not (`self.IsPainted`))
            (`PrimitiveComponent.SetMaterial` (`Character.Mesh` _asbp_cube) 0 "/Engine/MapTemplates/Materials/BasicAsset03.BasicAsset03")
            (set `/Game/BP_Cube.IsPainted` false _asbp_cube)))
        (:`CastFailed`
          (bind _asbp_clear_cube (cast `/Game/BP_ClearCube` Other))
          (if (not (`/Game/BP_ClearCube.IsPainted` _asbp_clear_cube))
            (`PrimitiveComponent.SetMaterial` (`self.Mesh`) 0 "/Engine/MapTemplates/Materials/BasicTemplateMaterial.BasicTemplateMaterial")
            (set `self.IsPainted` false)))))))

(fn `UserConstructionScript`)